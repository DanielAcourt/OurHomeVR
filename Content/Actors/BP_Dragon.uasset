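; BP_Dragon is a dragon actor Blueprint that, as it stands, only runs a debug line trace test.
; Each Tick it traces on the Camera channel with timed debug drawing and prints a message when something is hit.
; The trace has no start or end supplied, and BeginPlay, overlap and the construction script add no behavior.
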(event EventBeginPlay
  (|CallParentFunction) ; This node is disabled and will not be called.\nDrag off pins to build functionality.
)

(event Collision|EventActorBeginOverlap
  (params (OtherActor :type Actor%20Object%20Reference))
  (|CallParentFunction OtherActor) ; This node is disabled and will not be called.\nDrag off pins to build functionality.
)

(event EventTick
  (params (DeltaSeconds :type Float%20%28single-precision%29))
  (|CallParentFunction DeltaSeconds)
  (bind _returnvalue (Collision|LineTraceByChannel "0, 0, 0" "0, 0, 0" "TraceTypeQuery2" false 0 "ForDuration"))
  (if _returnvalue
    (Development|PrintString (Utilities|String|Append "I hit something" ""))))

(fn ConstructionScript
  (|CallParentFunction))
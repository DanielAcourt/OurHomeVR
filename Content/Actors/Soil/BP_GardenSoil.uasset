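; Garden soil actor that holds fertility, density and Qi stats in its components, as an unfinished prototype.
; GardenUpdate switches on the SaveableEntity's focus: Qi grows by its per-second rate unclamped, and fertility rolls over at its max, raising that cap.
; Density and below-cap fertility updates currently add zero.
; Random stat seeding exists but its BeginPlay hookup is disconnected, and gameplay-tag sub-typing is only unwired experiments.
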(event OnComponentActivated(SaveableEntity)
  (params (Component :type Actor%20Component%20Object%20Reference) (bReset :type Boolean)))

(event EventBeginPlay
  (|CallParentFunction))

(event Collision|EventActorBeginOverlap
  (params (OtherActor :type Actor%20Object%20Reference))
  (|CallParentFunction OtherActor) ; This node is disabled and will not be called.\nDrag off pins to build functionality.
)

(event EventTick
  (params (DeltaSeconds :type Float%20%28single-precision%29))
  (|CallParentFunction DeltaSeconds) ; This node is disabled and will not be called.\nDrag off pins to build functionality.
)

(fn ConstructionScript
  (|CallParentFunction))

(fn SpawnRandominRange
  (params (MinFertility :type Float%20%28double-precision%29) (MaxFertility :type Float%20%28double-precision%29) (MinDensity :type Float%20%28double-precision%29) (MaxDensity :type Float%20%28double-precision%29) (MinQi :type Float%20%28double-precision%29) (MaxQi :type Float%20%28double-precision%29))
  ;[0.15 0.15 0.15 0.5] Gets Random Numbers on spawn and set them to its data structure
  (Variables|/Script/WispsCpp.SoilDataComponent|SetSoilData (Variables|Default|GetSoilData) (Utilities|Struct|MakeSoilData "0001.01.01-00.00.00" (Math|Random|RandomFloatinRange MinFertility MaxFertility) 0.0 (Math|Random|RandomFloatinRange MinDensity MaxDensity)))
  (Variables|/Script/WispsCpp.QiComponent|SetQiData (Variables|Default|GetQi) (Utilities|Struct|MakeQiData MinQi (Math|Random|RandomFloatinRange MinQi MaxQi) 1.0))
  (return))

(fn GardenUpdate
  ;[0.03425 0.15 0 0.5] Using enum swithc for logic
  (switch Utilities|FlowControl|Switch|SwitchonETrainingFocus (Variables|/Script/WispsCpp.SaveableEntityComponent|GetCurrentFocus (Variables|Default|GetSaveableEntity))
    (:TF_Qi
      (CallFunction|UpdateQi))
    (:TF_Strength
      (CallFunction|UpdateDensity))
    (:TF_Dexterity
      (CallFunction|UpdateFertility))))

(fn AssignSubTags
  (params (SavableEntity :type Entity%20Save%20Data%20Structure)))

(fn UpdateQi
  (Variables|/Script/WispsCpp.QiComponent|SetQiData (Variables|Default|GetQi) (Utilities|Struct|MakeQiData (+ (.currentqi (Variables|/Script/WispsCpp.QiComponent|GetQiData (Variables|Default|GetQi))) (.baseqipersecond (Variables|/Script/WispsCpp.QiComponent|GetQiData (Variables|Default|GetQi)))) (.maxqi (Variables|/Script/WispsCpp.QiComponent|GetQiData (Variables|Default|GetQi))) (.baseqipersecond (Variables|/Script/WispsCpp.QiComponent|GetQiData (Variables|Default|GetQi)))))
  (return))

(fn UpdateFertility
  (if (>= (.fertility (Variables|/Script/WispsCpp.SoilDataComponent|GetSoilData (Variables|Default|GetSoilData))) (.fertilitymax (Variables|/Script/WispsCpp.SoilDataComponent|GetSoilData (Variables|Default|GetSoilData))))
    (Variables|/Script/WispsCpp.SoilDataComponent|SetSoilData (Variables|Default|GetSoilData) (Utilities|Struct|MakeSoilData (.lastupdatetime (Variables|/Script/WispsCpp.SoilDataComponent|GetSoilData (Variables|Default|GetSoilData))) (- (.fertility (Variables|/Script/WispsCpp.SoilDataComponent|GetSoilData (Variables|Default|GetSoilData))) (.fertilitymax (Variables|/Script/WispsCpp.SoilDataComponent|GetSoilData (Variables|Default|GetSoilData)))) (+ (.fertilitymax (Variables|/Script/WispsCpp.SoilDataComponent|GetSoilData (Variables|Default|GetSoilData))) 1.0) (.density (Variables|/Script/WispsCpp.SoilDataComponent|GetSoilData (Variables|Default|GetSoilData))) (.densitymax (Variables|/Script/WispsCpp.SoilDataComponent|GetSoilData (Variables|Default|GetSoilData))) 0.0 0.0 0.0 (.soilstatetag (Variables|/Script/WispsCpp.SoilDataComponent|GetSoilData (Variables|Default|GetSoilData)))))
    (else
      (Variables|/Script/WispsCpp.SoilDataComponent|SetSoilData (Variables|Default|GetSoilData) (Utilities|Struct|MakeSoilData (.lastupdatetime (Variables|/Script/WispsCpp.SoilDataComponent|GetSoilData (Variables|Default|GetSoilData))) (+ (.fertility (Variables|/Script/WispsCpp.SoilDataComponent|GetSoilData (Variables|Default|GetSoilData))) 0.0) (.fertilitymax (Variables|/Script/WispsCpp.SoilDataComponent|GetSoilData (Variables|Default|GetSoilData))) (.density (Variables|/Script/WispsCpp.SoilDataComponent|GetSoilData (Variables|Default|GetSoilData))) 0.0 0.0 0.0 0.0 (.soilstatetag (Variables|/Script/WispsCpp.SoilDataComponent|GetSoilData (Variables|Default|GetSoilData))))))))

(fn UpdateDensity
  (Variables|/Script/WispsCpp.SoilDataComponent|SetSoilData (Variables|Default|GetSoilData) (Utilities|Struct|MakeSoilData (Math|DateTime|Now) (.fertility (Variables|/Script/WispsCpp.SoilDataComponent|GetSoilData (Variables|Default|GetSoilData))) (.fertilitymax (Variables|/Script/WispsCpp.SoilDataComponent|GetSoilData (Variables|Default|GetSoilData))) (+ (.density (Variables|/Script/WispsCpp.SoilDataComponent|GetSoilData (Variables|Default|GetSoilData))) 0.0) (.densitymax (Variables|/Script/WispsCpp.SoilDataComponent|GetSoilData (Variables|Default|GetSoilData))) 0.0 0.0 0.0 (.soilstatetag (Variables|/Script/WispsCpp.SoilDataComponent|GetSoilData (Variables|Default|GetSoilData))))))